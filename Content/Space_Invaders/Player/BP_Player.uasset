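; Player pawn for a Space Invaders game that slides along X and fires only when its previous projectile is gone.
; Enemy deaths award score reduced by the Miss count, restore a life every eighth kill up to three, and trigger a win when no enemies remain.
; TakeHit spends lives until a loss; winning drives a timeline that moves the ship along Y, and both outcomes open MainMap.
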(event Custom|WIN
  (Development|PrintString "win" true true "(R=0.712124,G=1.000000,B=0.000000,A=1.000000)")
  (Variables|Default|Setlastloc (Transformation|GetActorLocation))
  (Components|Timeline|SetPlayRate (Variables|Default|Getendmove) 0.5)
  (bind _newtrack_0 (Timeline|endmove Play)
    (:Update
      (Transformation|SetActorLocation (Math|Vector|Lerp(Vector) (Variables|Default|Getlastloc) (+ (Variables|Default|Getlastloc) "0,1000.000000, 0") _newtrack_0) false false)
      (Game|OpenLevel(byName) "MainMap"))))

(event Custom|LOSE
  (Development|PrintString "lose" true true "(R=1.000000,G=0.000000,B=0.160864,A=1.000000)")
  (Utilities|FlowControl|Delay 1.0)
  (Game|OpenLevel(byName) "MainMap"))

(event EventTakeHit
  (if (== (Variables|Default|Getlives) 0)
    (CallFunction|LOSE)
    (else
      (Variables|Default|Setlives (- (Variables|Default|Getlives) 1)))))

(event Input|ActionEvents|InputActionShoot
  (params (Key :type Key%20Structure :default "None"))
  (:Pressed
    (Utilities|IsValid (Variables|Default|GetLastProjectile)
      (:Is%20Not%20Valid
        (bind _returnvalue (Game|SpawnActorfromClass "/Game/Space_Invaders/Projectile/Projectile.Projectile_C" (Transformation|GetWorldTransform (Variables|Default|GetArrow)) "AlwaysSpawn" 0 0))
        (Variables|Default|SetLastProjectile _returnvalue)))))

(event Input|AxisEvents|InputAxisMove
  (params (AxisValue :type Float%20%28single-precision%29))
  ;[1 1 1] Movement
  (Transformation|AddActorWorldOffset (* "1.000000,0.000000, 0" (* AxisValue (Utilities|Time|GetWorldDeltaSeconds) (Variables|Default|Getspeed))) true))

(fn ConstructionScript)

(fn OnEnemyDeath
  (CallFunction|DoScoreMath)
  (CallFunction|IsGameOver)
  (Variables|Default|Setmiss 0))

(fn DoScoreMath
  (Variables|Default|Setscore (+ (Variables|Default|Getscore) (- 100 (* 5 (Math|Integer|Min(Integer) 10 (Variables|Default|Getmiss))))))
  (Variables|Default|Setkills (+ (Variables|Default|Getkills) 1))
  (if (== (Math|Integer|%(Integer) (Variables|Default|Getkills) 8) 0)
    (Variables|Default|Setlives (Math|Integer|Min(Integer) (+ (Variables|Default|Getlives) 1) 3))))

(fn IsGameOver
  (bind _outactors (Actor|GetAllActorsOfClass "/Game/Space_Invaders/Enemy/Enemy.Enemy_C"))
  (if (== (Utilities|Array|Length _outactors) 0)
    (CallFunction|WIN)))